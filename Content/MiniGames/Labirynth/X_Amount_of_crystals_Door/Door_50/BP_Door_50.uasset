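; Sliding door for the Labyrinth minigame's crystal-count doors, driven by Button_50 actors.
; On BeginPlay it finds Button_50 actors by class and binds its Open and Close events to their dispatchers.
; Open moves the Cube 600 units below WorldLocation over one second, and Close moves it to WorldLocation.
; Both moves pass world location and rotation as relative targets to MoveComponentTo.
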(event `self.ReceiveBeginPlay`
  (bind _outactors (`GameplayStatics.GetAllActorsOfClass` "/Game/MiniGames/Labirynth/X_Amount_of_crystals_Door/Door_50/Button_50.Button_50_C"))
  (add `/Game/MiniGames/Labirynth/X_Amount_of_crystals_Door/Door_50/Button_50.Open` _outactors (delegate `Open`))
  (add `/Game/MiniGames/Labirynth/X_Amount_of_crystals_Door/Door_50/Button_50.Close` _outactors (delegate `Close`)))

(event `Open`
  (`KismetSystemLibrary.MoveComponentTo` (`self.Cube`) (- (`self.World Location`) (0.0 0.0 600.0)) (`self.WorldRotation`) false false 1.0))

(event `Close`
  (`KismetSystemLibrary.MoveComponentTo` (`self.Cube`) (`self.World Location`) (`self.WorldRotation`) false false 1.0))

(fn `UserConstructionScript`)