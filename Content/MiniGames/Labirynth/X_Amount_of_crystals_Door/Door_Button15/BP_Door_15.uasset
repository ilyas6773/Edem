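; BP_Door_15 is a door in the Labirynth minigame that opens and closes in response to Button_15 actors.
; On BeginPlay it finds those actors by class and binds their Open and Close dispatchers to its own events.
; Open slides the Door component down with MoveComponentTo, computing the relative target from world location.
; Close moves it to a hard-coded position, so the asset is tied to one placement.
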(event `self.ReceiveBeginPlay`
  (bind _outactors (`GameplayStatics.GetAllActorsOfClass` "/Game/MiniGames/Labirynth/X_Amount_of_crystals_Door/Door_Button15/Button_15.Button_15_C"))
  (add `/Game/MiniGames/Labirynth/X_Amount_of_crystals_Door/Door_Button15/Button_15.Open` _outactors (delegate `Open`))
  (add `/Game/MiniGames/Labirynth/X_Amount_of_crystals_Door/Door_Button15/Button_15.Close` _outactors (delegate `Close`)))

(event `Open`
  (bind _door (`self.Door`))
  (`KismetSystemLibrary.MoveComponentTo` _door (- (`SceneComponent.K2_GetComponentLocation` _door) (0.0 0.0 1000.0)) (`SceneComponent.K2_GetComponentRotation` _door) false false 0.5))

(event `Close`
  (`KismetSystemLibrary.MoveComponentTo` (`self.Door`) (10110.0 -3300.0 -40.0) (`SceneComponent.K2_GetComponentRotation` (`self.Door`)) false false 0.5))

(fn `UserConstructionScript`)