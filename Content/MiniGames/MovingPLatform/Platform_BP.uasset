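; Moving platform Blueprint that travels along waypoints using an InterpToMovement component.
; The construction script copies the WayPoints and Duration variables into the component and turns off its auto-activation.
; PP_Activated activates the movement and enables its tick.
; PP_Deactivated disables the tick to halt the platform while leaving the component active and without resetting it.
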(event `PP_Activated`
  (bind _interptomovement (`self.InterpToMovement`))
  (`ActorComponent.SetActive` _interptomovement true false)
  (`ActorComponent.SetComponentTickEnabled` _interptomovement true))

(event `PP_Deactivated`
  (bind _interptomovement (`self.InterpToMovement`))
  (`ActorComponent.SetActive` _interptomovement true false)
  (`ActorComponent.SetComponentTickEnabled` _interptomovement false))

(fn `UserConstructionScript`
  (bind _interptomovement (`self.InterpToMovement`))
  (set `InterpToMovementComponent.ControlPoints` (`self.WayPoints`) _interptomovement)
  (set `InterpToMovementComponent.Duration` (`self.Duration`) _interptomovement)
  (`ActorComponent.SetAutoActivate` _interptomovement false))