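; Base dark energy projectile for minigames that flies toward an optional target and reports its impact.
; The construction script applies speed and gravity to ProjectileMovement and can flag it as homing, though no homing target component is assigned here.
; BeginPlay aims velocity once at a valid target.
; A box hit calls the impact notification, spawns the impact effect and destroys the actor.
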(event `self.ReceiveBeginPlay`
  (`self.Target`
    (:`then`
      (`self.Rotate Target`))
    (:`else`)))

(event `RotateTarget`
  (set `MovementComponent.Velocity` (* (`KismetMathLibrary.GetDirectionUnitVector` (`self.K2_GetActorLocation`) (`self.K2_GetActorLocation` (`self.Target`))) (`self.Speed`)) (`self.ProjectileMovement`)))

(event `self.BoxCollision.OnComponentHit`
  (params (HitComponent :type "PrimitiveComponent Object Reference") (OtherActor :type "Actor Object Reference") (OtherComp :type "PrimitiveComponent Object Reference") (NormalImpulse :type "Vector Structure") (Hit :type "HitResult Structure (by ref)"))
  (`self.OnProjectileImpact` OtherActor Hit)
  (`GameplayStatics.SpawnEmitterAtLocation` (`self.ImpactEffect`) (`.Location` (`GameplayStatics.BreakHitResult` Hit)))
  (`self.K2_DestroyActor`))

(fn `Rotate Target`)

(fn `UserConstructionScript`
  (bind _projectilemovement (`self.ProjectileMovement`))
  (set `ProjectileMovementComponent.InitialSpeed` (`self.Speed`) _projectilemovement)
  (set `ProjectileMovementComponent.MaxSpeed` (`self.Speed`) _projectilemovement)
  (set `ProjectileMovementComponent.ProjectileGravityScale` (`self.Gravity`) _projectilemovement)
  (`self.Target`
    (:`then`
      (if (`self.IsHoming_0`)
        (set `ProjectileMovementComponent.bIsHomingProjectile` true _projectilemovement)))
    (:`else`)))