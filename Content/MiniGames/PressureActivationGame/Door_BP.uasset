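; Door for the pressure activation minigame that moves vertically once enough pressure switches are active.
; SwitchActivated and SwitchDeactivated events raise and lower a count of active switches, which is compared to the required number.
; A Timeline drives the Door component's relative Z location, playing when the threshold is met and reversing when the count drops below it.
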(event `SwitchActivated`
  (`/Engine/EditorBlueprintResources/StandardMacros.IncrementInt` (`self.PressureSwitchesActive`)
    (:`  `
      (if (>= (`self.PressureSwitchesActive`) (`self.SwitchersPressureNeeded`))
        (bind (_direction _newtrack_0) (`Timeline|Timeline` :!label _label)
          (:`Update`
            (`SceneComponent.K2_SetRelativeLocation` (`self.Door`) (`KismetMathLibrary.MakeVector` 0.0 0.0 _newtrack_0) false false)))))))

(event `SwitchDeactivated`
  (`/Engine/EditorBlueprintResources/StandardMacros.DecrementInt` (`self.PressureSwitchesActive`)
    (:`  `
      (if (not (>= (`self.PressureSwitchesActive`) (`self.SwitchersPressureNeeded`)))
        (goto _label :!via `Reverse`)))))

(fn `UserConstructionScript`)