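; Enemy AI character that wanders the navmesh, chaining random move requests from BeginPlay each time one succeeds.
; PawnSensing sightings pass a DoOnce that switches to a jog animation at sprint speed, and also issue an AI move with no destination wired.
; A retriggerable delay drops it to a slow walk once sightings lapse.
; CanSprintAgain resets the sprint gate but is not called here.
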(event `self.ReceiveBeginPlay`
  (`self.MoveToRandomLocation`))

(event `MoveToRandomLocation`
  (bind _randomlocation (`NavigationSystemV1.K2_GetRandomLocationInNavigableRadius` (`self.K2_GetActorLocation`) 0.0 null null))
  (`|AIMoveTo` self _randomlocation null
    (:`OnSuccess`
      (`self.MoveToRandomLocation`))))

(event `CanSprintAgain`
  (goto _label :!via `Reset`))

(event `self.PawnSensing.OnSeePawn`
  (params (Pawn :type "Pawn Object Reference"))
  (`|ExecutionSequence`
    (:`then_0`
      (`/Engine/EditorBlueprintResources/StandardMacros.DoOnce` false :!label _label
        (:`Completed`
          (`SkeletalMeshComponent.PlayAnimation` (`self.Mesh`) "/Game/Characters/Mannequin_UE4/Animations/Jog_Fwd.Jog_Fwd" false)
          (set `CharacterMovementComponent.MaxWalkSpeed` 600.0 (`self.CharacterMovement`)))))
    (:`then_1`
      (`|AIMoveTo` self (0.0 0.0 0.0) null
        (:`then`
          (`KismetSystemLibrary.RetriggerableDelay` 5.0)
          (`SkeletalMeshComponent.PlayAnimation` (`self.Mesh`) null false)
          (set `CharacterMovementComponent.MaxWalkSpeed` 100.0 (`self.CharacterMovement`)))))))

(fn `UserConstructionScript`)